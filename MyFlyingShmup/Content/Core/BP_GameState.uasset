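; Game state Blueprint that tracks level completion across all wave managers and provides player pawn spawning.
; On BeginPlay it plays a 2D sound and binds to each BP_WaveManager's all-waves-ended announcement.
; Once every manager has reported, it calls LevelComplete, which is empty here.
; SpawnPlayerPawn, not called here, spawns the game mode's default pawn at a PlayerStart and possesses it with player controller 0.
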(event Custom|SpawnPlayerPawn
  (bind _returnvalue (Actor|GetActorOfClass "/Script/Engine.PlayerStart"))
  (bind _returnvalue_2 (Game|SpawnActorfromClass (Variables|/Script/Engine.GameModeBase|GetDefaultPawnClass (Game|GetGameMode)) (Transformation|GetActorTransform _returnvalue) "AlwaysSpawn" "MultiplyWithRoot" 0 0))
  (Pawn|Possess (Game|GetPlayerController 0) _returnvalue_2))

(event Custom|AWaveHasEnded
  (bind _result (Math|Integer|IncrementInt (Variables|Default|GetTotalNumberOfWaveManagersThatHaveEnded))
    (:%20%20
      (if (== _result (Variables|Default|GetTotalNumberOfWaveManagers))
        (CallFunction|LevelComplete)))))

(event Custom|LevelComplete)

(event EventBeginPlay
  (Audio|PlaySound2D "/Game/Tri_Sky_Audio/Tri_Sky_01.Tri_Sky_01" 1.0 1.0 0.0 0 0)
  (bind _outactors (Actor|GetAllActorsOfClass "/Game/Blueprints/BP_WaveManager.BP_WaveManager_C"))
  (Variables|Default|SetTotalNumberOfWaveManagers (Utilities|Array|Length _outactors))
  (for _array_element _outactors
    (EventDispatchers|BindEventtoAnnounceAllWavesHaveEnded _array_element (delegate Custom|AWaveHasEnded))))

(fn ConstructionScript)