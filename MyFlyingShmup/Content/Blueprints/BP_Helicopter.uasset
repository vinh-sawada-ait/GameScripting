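; Player-controlled helicopter pawn that moves along world X and Y axes through Enhanced Input and a FloatingPawnMovement component.
; On Tick it banks by interpolating roll toward a left or right tilt, leveling out when both or neither side input is held.
; Three RotatingMovement components, bound to sphere components on BeginPlay, spin the rotors; an older Tick-based rotor spin is left disconnected.
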(event Input|EnhancedActionEvents|EnhancedInputActionIA_MoveForward
  (params (ActionValue :type Boolean) (ElapsedSeconds :type Float%20%28double-precision%29) (TriggeredSeconds :type Float%20%28double-precision%29) (InputAction :type Input%20Action%20Object%20Reference :default "/Game/Inputs/IA_MoveForward.IA_MoveForward"))
  (Class|PawnMovementComponent|AddInputVector (Variables|Default|GetFloatingPawnMovement) "1.000000,0.000000,0.000000" false))

(event Input|EnhancedActionEvents|EnhancedInputActionIA_MoveBackward
  (params (ActionValue :type Boolean) (ElapsedSeconds :type Float%20%28double-precision%29) (TriggeredSeconds :type Float%20%28double-precision%29) (InputAction :type Input%20Action%20Object%20Reference :default "/Game/Inputs/IA_MoveBackward.IA_MoveBackward"))
  (Class|PawnMovementComponent|AddInputVector (Variables|Default|GetFloatingPawnMovement) "-1.000000,0.000000,0.000000" false))

(event Input|EnhancedActionEvents|EnhancedInputActionIA_MoveLeft
  (params (ActionValue :type Boolean) (ElapsedSeconds :type Float%20%28double-precision%29) (TriggeredSeconds :type Float%20%28double-precision%29) (InputAction :type Input%20Action%20Object%20Reference :default "/Game/Inputs/IA_MoveLeft.IA_MoveLeft"))
  (Class|PawnMovementComponent|AddInputVector (Variables|Default|GetFloatingPawnMovement) "0.000000,-1.000000,0.000000" false))

(event Input|EnhancedActionEvents|EnhancedInputActionIA_MoveRight
  (params (ActionValue :type Boolean) (ElapsedSeconds :type Float%20%28double-precision%29) (TriggeredSeconds :type Float%20%28double-precision%29) (InputAction :type Input%20Action%20Object%20Reference :default "/Game/Inputs/IA_MoveRight.IA_MoveRight"))
  (Class|PawnMovementComponent|AddInputVector (Variables|Default|GetFloatingPawnMovement) "0.000000,1.000000,0.000000" false))

(event EventTick
  (params (DeltaSeconds :type Float%20%28single-precision%29))
  (bind _returnvalue (Input|EnhancedActionValues|GetIA_MoveLeft))
  (bind _returnvalue_2 (Input|EnhancedActionValues|GetIA_MoveRight))
  (bind _output_get (Variables|Default|SetDelta%20Seconds DeltaSeconds))
  (bind _output_get_2 (Variables|Default|SetCurrent%20Rotation (Math|Interpolation|FInterpTo (Variables|Default|GetCurrent%20Rotation) (Variables|Default|GetTarget%20Rotation) _output_get 4.0)))
  (Transformation|SetActorRotation (Math|Rotator|MakeRotator (* _output_get_2 3e+01) 0.0 0.0))
  (Variables|Default|SetTarget%20Rotation (Math|Float|SelectFloat 0.0 (Math|Float|SelectFloat -1.0 1.0 (Input|EnhancedActionValues|GetIA_MoveLeft)) (or (and _returnvalue_2 _returnvalue) (Math|Boolean|NORBoolean _returnvalue_2 _returnvalue)))))

(event EventBeginPlay
  ;[0.15 0.15 0.15 0.5] Rotate Rotors using ROTATING COMPONENT
  (Components|Movement|SetUpdatedComponent (Variables|Default|GetRotatingMovement) (Variables|Default|GetSphere1))
  (Components|Movement|SetUpdatedComponent (Variables|Default|GetRotatingMovement1) (Variables|Default|GetSphere2))
  (Components|Movement|SetUpdatedComponent (Variables|Default|GetRotatingMovement2) (Variables|Default|GetSphere3)))

(event EventPossessed
  (params (NewController :type Controller%20Object%20Reference))
  (bind _asplayer_controller (Utilities|Casting|CastToPlayerController NewController))
  (Input|AddMappingContext (PlayerController|LocalPlayerSubsystems|GetEnhancedInputLocalPlayerSubsystem _asplayer_controller) "/Game/Inputs/IMC_PlayerMovement.IMC_PlayerMovement" 0 "(bIgnoreAllPressedKeysUntilRelease=True,bForceImmediately=False,bNotifyUserSettings=False)"))

(fn ConstructionScript)