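; BP_Pickup_Health is a health pickup that heals the player pawn on overlap.
; When an overlapping actor casts to BP_PlayerPawn, it adds a fixed amount to the pawn's current health, clamped to its maximum.
; The pickup then destroys itself, even if the player is already at full health.
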(event EventBeginPlay
  (|CallParentFunction) ; This node is disabled and will not be called.\nDrag off pins to build functionality.
)

(event Collision|EventActorBeginOverlap
  (params (OtherActor :type Actor%20Object%20Reference))
  (bind _asbp_player_pawn (Utilities|Casting|CastToBP_PlayerPawn OtherActor))
  (Variables|/Game/Blueprints/BP_PlayerPawn.BP_PlayerPawn_C|SetCurrentPlayerHealth _asbp_player_pawn (Math|Float|Min(Float) (+ (Variables|/Game/Blueprints/BP_PlayerPawn.BP_PlayerPawn_C|GetCurrentPlayerHealth _asbp_player_pawn) 5e+01) (Variables|/Game/Blueprints/BP_PlayerPawn.BP_PlayerPawn_C|GetMaxPlayerHealth _asbp_player_pawn)))
  (Actor|DestroyActor))

(fn ConstructionScript
  (|CallParentFunction))