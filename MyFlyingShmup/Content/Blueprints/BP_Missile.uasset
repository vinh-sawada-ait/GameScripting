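; BP_Missile is a missile actor that flies along an animated path after it spawns.
; On BeginPlay it stores its spawn location and plays a timeline that offsets it from that point each update.
; The timeline drives forward travel on world X and a sideways Y curve, mirrored by the RightSideSpawn flag.
; Movement sets the location directly without sweep, ignoring the actor's facing.
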(event EventBeginPlay
  (Variables|Default|SetInitialLocation (Transformation|GetActorLocation))
  (bind (_direction _y_value _x_value) (Timeline|Timeline PlayFromStart)
    (:Update
      (Transformation|SetActorLocation (+ (Math|Vector|MakeVector (* _x_value 8e+03) (* _y_value (Math|Float|SelectFloat 4e+02 -4e+02 (Variables|Default|GetRightSideSpawn))) 0.0) (Variables|Default|GetInitialLocation)) false false))))

(fn ConstructionScript)