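; Player ship pawn that moves on a plane, banks when strafing and fires projectiles.
; Enhanced Input drives FloatingPawnMovement, while Tick eases roll toward the strafe direction.
; A debug key cycles fire modes: cooldown-gated twin bullets, cooldown-gated missiles alternating sides via FlipFlop, or an ungated bullet fan.
; Possession creates the HUD; any actor overlap deals fixed damage and updates its health widget, with death only printed.
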(event Custom|SwitchShootingMode
  (bind _output_get (Variables|Default|SetShootingMode (Math|Integer|%(Integer) (+ (Variables|Default|GetShootingMode) 1) (+ (Variables|Default|GetMaxShootingMode) 1))))
  (Development|PrintString (Utilities|String|ToString(Integer) _output_get)))

(event Input|EnhancedActionEvents|EnhancedInputActionIA_MoveForward
  (params (ActionValue :type Boolean) (ElapsedSeconds :type Float%20%28double-precision%29) (TriggeredSeconds :type Float%20%28double-precision%29) (InputAction :type Input%20Action%20Object%20Reference :default "/Game/Inputs/IA_MoveForward.IA_MoveForward"))
  (Class|PawnMovementComponent|AddInputVector (Variables|Default|GetFloatingPawnMovement) "1.000000,0.000000,0.000000" false))

(event Input|EnhancedActionEvents|EnhancedInputActionIA_MoveBackward
  (params (ActionValue :type Boolean) (ElapsedSeconds :type Float%20%28double-precision%29) (TriggeredSeconds :type Float%20%28double-precision%29) (InputAction :type Input%20Action%20Object%20Reference :default "/Game/Inputs/IA_MoveBackward.IA_MoveBackward"))
  (Class|PawnMovementComponent|AddInputVector (Variables|Default|GetFloatingPawnMovement) "-1.000000,0.000000,0.000000" false))

(event Input|EnhancedActionEvents|EnhancedInputActionIA_MoveLeft
  (params (ActionValue :type Boolean) (ElapsedSeconds :type Float%20%28double-precision%29) (TriggeredSeconds :type Float%20%28double-precision%29) (InputAction :type Input%20Action%20Object%20Reference :default "/Game/Inputs/IA_MoveLeft.IA_MoveLeft"))
  (Class|PawnMovementComponent|AddInputVector (Variables|Default|GetFloatingPawnMovement) "0.000000,-1.000000,0.000000" false))

(event Input|EnhancedActionEvents|EnhancedInputActionIA_MoveRight
  (params (ActionValue :type Boolean) (ElapsedSeconds :type Float%20%28double-precision%29) (TriggeredSeconds :type Float%20%28double-precision%29) (InputAction :type Input%20Action%20Object%20Reference :default "/Game/Inputs/IA_MoveRight.IA_MoveRight"))
  (Class|PawnMovementComponent|AddInputVector (Variables|Default|GetFloatingPawnMovement) "0.000000,1.000000,0.000000" false))

(event Input|EnhancedActionEvents|EnhancedInputActionIA_PrimaryFire
  (params (ActionValue :type Boolean) (ElapsedSeconds :type Float%20%28double-precision%29) (TriggeredSeconds :type Float%20%28double-precision%29) (InputAction :type Input%20Action%20Object%20Reference :default "/Game/Inputs/IA_PrimaryFire.IA_PrimaryFire"))
  (bind _primaryfirespawnpoint (Variables|Default|GetPrimaryFireSpawnPoint))
  (bind _sphere2 (Variables|Default|GetSphere2))
  (bind _returnvalue (Transformation|GetWorldLocation _primaryfirespawnpoint))
  (bind _returnvalue_2 (Transformation|GetWorldLocation _sphere2))
  (switch int (Variables|Default|GetShootingMode)
    (:0
      (Utilities|FlowControl|DoOnce false :!label _label
        (:Completed
          (Game|SpawnActorfromClass "/Game/Blueprints/BP_Bullet.BP_Bullet_C" (Math|Transform|MakeTransform (+ _returnvalue "0.000000,50.000000,0.000000") "0, 0, 0" "1.000000,1.000000,1.000000") "Undefined" "MultiplyWithRoot" 0 0)
          (Game|SpawnActorfromClass "/Game/Blueprints/BP_Bullet.BP_Bullet_C" (Math|Transform|MakeTransform (+ _returnvalue "0.000000,-50.000000,0.000000") "0, 0, 0" "1.000000,1.000000,1.000000") "Undefined" "MultiplyWithRoot" 0 0)
          (Utilities|FlowControl|Delay 0.2)
          (goto _label Reset))))
    (:1
      (Utilities|FlowControl|DoOnce false :!label _label_2
        (:Completed
          (Utilities|FlowControl|FlipFlop
            (:A
              (Game|SpawnActorfromClass "/Game/Blueprints/BP_Missile.BP_Missile_C" (Math|Transform|MakeTransform _returnvalue_2 "0, 0, 0" "1.000000,1.000000,1.000000") "Undefined" "MultiplyWithRoot" 0 true 0))
            (:B
              (Game|SpawnActorfromClass "/Game/Blueprints/BP_Missile.BP_Missile_C" (Math|Transform|MakeTransform _returnvalue_2 "0, 0, 0" "1.000000,1.000000,1.000000") "Undefined" "MultiplyWithRoot" 0 false 0)))
          (Utilities|FlowControl|Delay 1.0)
          (goto _label_2 Reset))))
    (:2
      (for _index (range 0 (- (Variables|Default|GetBullets) 1))
        (Game|SpawnActorfromClass "/Game/Blueprints/BP_Bullet.BP_Bullet_C" (Math|Transform|MakeTransform (Transformation|GetWorldLocation (Variables|Default|GetPrimaryFireSpawnPoint)) (Math|Rotator|MakeRotator 0.0 0.0 (Utilities|Operators|Subtract (* _index 1e+01) (* (Variables|Default|GetBullets) 5) -5.0)) "1.000000,1.000000,1.000000") "Undefined" "MultiplyWithRoot" 0 0)))))

(event EventTick
  (params (DeltaSeconds :type Float%20%28single-precision%29))
  (bind _returnvalue (Input|EnhancedActionValues|GetIA_MoveLeft))
  (bind _returnvalue_2 (Input|EnhancedActionValues|GetIA_MoveRight))
  (bind _output_get (Variables|Default|SetDelta%20Seconds DeltaSeconds))
  (bind _output_get_2 (Variables|Default|SetCurrent%20Rotation (Math|Interpolation|FInterpTo (Variables|Default|GetCurrent%20Rotation) (Variables|Default|GetTarget%20Rotation) _output_get 4.0)))
  (Transformation|SetActorRotation (Math|Rotator|MakeRotator (* _output_get_2 3e+01) 0.0 0.0))
  (Variables|Default|SetTarget%20Rotation (Math|Float|SelectFloat 0.0 (Math|Float|SelectFloat -1.0 1.0 (Input|EnhancedActionValues|GetIA_MoveLeft)) (or (and _returnvalue_2 _returnvalue) (Math|Boolean|NORBoolean _returnvalue_2 _returnvalue)))))

(event EventPossessed
  (params (NewController :type Controller%20Object%20Reference))
  (bind _asplayer_controller (Utilities|Casting|CastToPlayerController NewController))
  (Input|AddMappingContext (PlayerController|LocalPlayerSubsystems|GetEnhancedInputLocalPlayerSubsystem _asplayer_controller) "/Game/Inputs/IMC_PlayerMovement.IMC_PlayerMovement" 0 "(bIgnoreAllPressedKeysUntilRelease=True,bForceImmediately=False,bNotifyUserSettings=False)")
  ;[0.7489 1 0] Add Base Widget
  (bind _returnvalue (UserInterface|CreateWidget "/Game/Ui/WBP_BaseWidget.WBP_BaseWidget_C"))
  (UserInterface|Viewport|AddtoViewport _returnvalue 0)
  (Variables|Default|SetWBP%20Player%20Health (Variables|/Game/Ui/WBP_BaseWidget.WBP_BaseWidget_C|GetWBP_PlayerHealth _returnvalue)))

(event Input|KeyboardEvents|DebugKeyCtrlT
  (params (Key :type Key%20Structure :default "None") (ActionValue :type Input%20Action%20Value%20Structure))
  (:Pressed
    (CallFunction|SwitchShootingMode)))

(event Collision|EventActorBeginOverlap
  (params (OtherActor :type Actor%20Object%20Reference))
  (Development|PrintString "I'm HIIIITTTT!!!!")
  (Variables|Default|SetCurrentPlayerHealth (- (Variables|Default|GetCurrentPlayerHealth) 25.0))
  (Default|SetHealth (Variables|Default|GetWBP%20Player%20Health) (/ (Variables|Default|GetCurrentPlayerHealth) (Variables|Default|GetMaxPlayerHealth)))
  (if (<= (Variables|Default|GetCurrentPlayerHealth) 0.0)
    (Development|PrintString "I'm DEAD!!!!")))

(fn ConstructionScript)